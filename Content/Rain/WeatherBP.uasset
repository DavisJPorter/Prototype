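; WeatherBP toggles the scene between bright sky and dark rainy weather on left mouse clicks, provided its sky reference is valid.
; A FlipFlop plays or reverses one Timeline that blends the sky material's zenith, horizon, cloud color and opacity, plus the light color.
; Delays stagger the referenced rain particle system: it activates after darkening starts, and deactivates before the sky begins to brighten.
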(event Input|MouseEvents|LeftMouseButton
  (params (Key :type Key%20Structure :default "None"))
  (bind _rain_ref (Variables|Default|GetRain_Ref))
  (bind _sky_ref (Variables|Default|GetSky_Ref))
  (bind _particlesystemcomponent (Variables|/Script/Engine.Emitter|GetParticleSystemComponent _rain_ref))
  (bind _sky_material (Variables|/Engine/EngineSky/BP_Sky_Sphere.BP_Sky_Sphere_C|GetSky%20material _sky_ref))
  (:Pressed
    (if (Utilities|IsValid (Variables|Default|GetSky_Ref))
      (Utilities|FlowControl|FlipFlop
        (:A
          (Utilities|FlowControl|Sequence
            (:then_0
              (bind _newtrack_0 (Timeline|Timeline_0 Play)
                (:Update
                  (Rendering|Material|SetVectorParameterValue _sky_material "Zenith" (Math|Color|Lerp(LinearColor) "(R=0.034046,G=0.109247,B=0.295000,A=1.000000)" "(R=0.052083,G=0.052083,B=0.052083,A=1.000000)" _newtrack_0) :!class /Script/Engine.MaterialInstanceDynamic)
                  (Rendering|Material|SetVectorParameterValue _sky_material "Horizon" (Math|Color|Lerp(LinearColor) "(R=1.979559,G=2.586644,B=3.000000,A=1.000000)" "(R=0.020833,G=0.020833,B=0.020833,A=1.000000)" _newtrack_0) :!class /Script/Engine.MaterialInstanceDynamic)
                  (Rendering|Material|SetVectorParameterValue _sky_material "Cloud" (Math|Color|Lerp(LinearColor) "(R=0.855778,G=0.919020,B=1.000000,A=1.000000)" "(R=0.041667,G=0.041667,B=0.041667,A=1.000000)" _newtrack_0) :!class /Script/Engine.MaterialInstanceDynamic)
                  (Rendering|Material|SetScalarParameterValue _sky_material "Cloud Opacity" (Math|Float|Lerp 1.2 0.5 _newtrack_0) :!class /Script/Engine.MaterialInstanceDynamic)
                  (Rendering|Components|Light|SetLightColor (Variables|/Script/Engine.Light|GetLightComponent (Variables|Default|GetLight_Ref)) (Math|Color|Lerp(LinearColor) "(R=0.855778,G=0.919020,B=1.000000,A=1.000000)" "(R=0.000000,G=0.000000,B=0.000000,A=1.000000)" _newtrack_0) true))))
            (:then_1
              (Utilities|FlowControl|Delay 5.0)
              (Components|Activation|Activate _particlesystemcomponent false))))
        (:B
          (Components|Activation|Deactivate _particlesystemcomponent)
          (Utilities|FlowControl|Delay 3.0)
          (Timeline|Timeline_0 Reverse))))))

(fn ConstructionScript)